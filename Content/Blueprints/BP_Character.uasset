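; BP_Character is a VR player character that moves relative to where the headset camera faces.
; On BeginPlay it sets the tracking origin to eye level and sets the actor's relative location from EyeHeight.
; The MoveForward and MoveRight axes feed movement input along the CameraVR forward and right vectors, with the forward axis inverted.
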(event `InputAxis|MoveForward`
  (params (AxisValue :type "Float (single-precision)"))
  ;[1 1 1] Movement
  (`self.AddMovementInput` (`SceneComponent.GetForwardVector` (`self.CameraVR`)) (* AxisValue -1.0)))

(event `self.ReceiveBeginPlay`
  ;[1 1 1] Set Camera Height
  (`HeadMountedDisplayFunctionLibrary.SetTrackingOrigin` "Eye")
  (`self.K2_SetActorRelativeLocation` (`self.EyeHeight`)))

(event `InputAxis|MoveRight`
  (params (AxisValue :type "Float (single-precision)"))
  ;[1 1 1] Movement
  (`self.AddMovementInput` (`SceneComponent.GetRightVector` (`self.CameraVR`)) AxisValue))

(fn `UserConstructionScript`)