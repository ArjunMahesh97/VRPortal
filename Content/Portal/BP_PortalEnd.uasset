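; BP_PortalEnd is a portal actor that teleports the player's BP_Character when it overlaps the collision box.
; On overlap it gathers all actors of a class, picks the one at index IntCount, and moves the character slightly above that actor's location.
; The character's forward vector is stored beforehand but not used afterward, and no rotation is supplied to the teleport.
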(event `self.CollisionBox.OnComponentBeginOverlap`
  (params (OverlappedComponent :type "PrimitiveComponent Object Reference") (OtherActor :type "Actor Object Reference") (OtherComp :type "PrimitiveComponent Object Reference") (OtherBodyIndex :type Integer) (bFromSweep :type Boolean) (SweepResult :type "HitResult Structure (by ref)"))
  (`|ExecutionSequence`
    (:`then_0`
      (bind _asbp_character (cast `/Game/Blueprints/BP_Character` OtherActor))
      (if true
        (bind _outactors (`GameplayStatics.GetAllActorsOfClass` null))
        (set `self.NewVar_0` (`self.GetActorForwardVector` _asbp_character))
        (bind (_returnvalue_x _returnvalue_y _returnvalue_z) (`KismetMathLibrary.BreakVector` (`self.K2_GetActorLocation` (`|GetArrayItem` _outactors (`self.IntCount`)))))
        (`self.K2_SetActorLocationAndRotation` :`self` _asbp_character :`NewLocation` (`KismetMathLibrary.MakeVector` _returnvalue_x _returnvalue_y (+ _returnvalue_z 50.0)))))))

(fn `UserConstructionScript`)